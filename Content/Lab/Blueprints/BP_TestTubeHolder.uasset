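; Lab test tube holder that fills itself with covered, filled and empty tubes from per-type counts.
; The Construction Script adds mesh instances to one component per tube type, placing covered, then filled, then empty tubes.
; A shared TubesPlaced counter and nested comparisons map each tube to five rows of ten, spaced along X by DistanceBetweenMeshes.
; The 50-tube total limit is only noted in a comment, not enforced.
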(event EventBeginPlay)

(event Collision|EventActorBeginOverlap
  (params (OtherActor :type Actor%20Object%20Reference)))

(event EventTick
  (params (DeltaSeconds :type Float%20%28single-precision%29)))

(fn ConstructionScript
  ;[1 1 1] Covered Tubes
  (for _index (range 1 (Variables|Default|GetNumberOfCoveredTubes))
    (bind _output_get (Variables|Default|SetTubesPlaced _index))
    (Math|Integer|CompareInt _output_get 10
      (:>
        (Math|Integer|CompareInt _output_get 20
          (:>
            (Math|Integer|CompareInt _output_get 30
              (:>
                (Math|Integer|CompareInt _output_get 40
                  (:>
                    (Components|InstancedStaticMesh|AddInstance (Variables|Default|GetCoveredTube) (Math|Transform|MakeTransform (Math|Vector|MakeVector (* (- (Variables|Default|GetTubesPlaced) 40) (Variables|Default|GetDistance%20Between%20Meshes)) 10.684 0.0)) false))
                  (:==
                    (Components|InstancedStaticMesh|AddInstance (Variables|Default|GetCoveredTube) (Math|Transform|MakeTransform (Math|Vector|MakeVector (* (- (Variables|Default|GetTubesPlaced) 30) (Variables|Default|GetDistance%20Between%20Meshes)) 8.013 0.0)) false :!label _label))
                  (:<
                    (goto _label))))
              (:==
                (Components|InstancedStaticMesh|AddInstance (Variables|Default|GetCoveredTube) (Math|Transform|MakeTransform (Math|Vector|MakeVector (* (- (Variables|Default|GetTubesPlaced) 20) (Variables|Default|GetDistance%20Between%20Meshes)) 5.342 0.0)) false :!label _label_2))
              (:<
                (goto _label_2))))
          (:==
            (Components|InstancedStaticMesh|AddInstance (Variables|Default|GetCoveredTube) (Math|Transform|MakeTransform (Math|Vector|MakeVector (* (- (Variables|Default|GetTubesPlaced) 10) (Variables|Default|GetDistance%20Between%20Meshes)) 2.671 0.0)) false :!label _label_3))
          (:<
            (goto _label_3))))
      (:==
        (Components|InstancedStaticMesh|AddInstance (Variables|Default|GetCoveredTube) (Math|Transform|MakeTransform (Math|Vector|MakeVector (* (Variables|Default|GetTubesPlaced) (Variables|Default|GetDistance%20Between%20Meshes)) 0.0 0.0)) false :!label _label_4))
      (:<
        (goto _label_4))))
  ;[1 1 1] Filled Tubes
  (for _index_2 (range 1 (Variables|Default|GetNumberOfFilledTubes))
    (bind _output_get_2 (Variables|Default|SetTubesPlaced (+ (Variables|Default|GetTubesPlaced) 1)))
    (Math|Integer|CompareInt _output_get_2 10
      (:>
        (Math|Integer|CompareInt _output_get_2 20
          (:>
            (Math|Integer|CompareInt _output_get_2 30
              (:>
                (Math|Integer|CompareInt _output_get_2 40
                  (:>
                    (Components|InstancedStaticMesh|AddInstance (Variables|Default|GetTestTubeFilled) (Math|Transform|MakeTransform (Math|Vector|MakeVector (* (- (Variables|Default|GetTubesPlaced) 40) (Variables|Default|GetDistance%20Between%20Meshes)) 10.684 0.0)) false))
                  (:==
                    (Components|InstancedStaticMesh|AddInstance (Variables|Default|GetTestTubeFilled) (Math|Transform|MakeTransform (Math|Vector|MakeVector (* (- (Variables|Default|GetTubesPlaced) 30) (Variables|Default|GetDistance%20Between%20Meshes)) 8.013 0.0)) false :!label _label_5))
                  (:<
                    (goto _label_5))))
              (:==
                (Components|InstancedStaticMesh|AddInstance (Variables|Default|GetTestTubeFilled) (Math|Transform|MakeTransform (Math|Vector|MakeVector (* (- (Variables|Default|GetTubesPlaced) 20) (Variables|Default|GetDistance%20Between%20Meshes)) 5.342 0.0)) false :!label _label_6))
              (:<
                (goto _label_6))))
          (:==
            (Components|InstancedStaticMesh|AddInstance (Variables|Default|GetTestTubeFilled) (Math|Transform|MakeTransform (Math|Vector|MakeVector (* (- (Variables|Default|GetTubesPlaced) 10) (Variables|Default|GetDistance%20Between%20Meshes)) 2.671 0.0)) false :!label _label_7))
          (:<
            (goto _label_7))))
      (:==
        (Components|InstancedStaticMesh|AddInstance (Variables|Default|GetTestTubeFilled) (Math|Transform|MakeTransform (Math|Vector|MakeVector (* (Variables|Default|GetTubesPlaced) (Variables|Default|GetDistance%20Between%20Meshes)) 0.0 0.0)) false :!label _label_8))
      (:<
        (goto _label_8))))
  ;[1 1 1] Empty Tubes
  (for _index_3 (range 1 (Variables|Default|GetNumberOfEmptyTubes))
    (bind _output_get_3 (Variables|Default|SetTubesPlaced (+ (Variables|Default|GetTubesPlaced) 1)))
    (Math|Integer|CompareInt _output_get_3 10
      (:>
        (Math|Integer|CompareInt _output_get_3 20
          (:>
            (Math|Integer|CompareInt _output_get_3 30
              (:>
                (Math|Integer|CompareInt _output_get_3 40
                  (:>
                    (Components|InstancedStaticMesh|AddInstance (Variables|Default|GetEmptyTube) (Math|Transform|MakeTransform (Math|Vector|MakeVector (* (- (Variables|Default|GetTubesPlaced) 40) (Variables|Default|GetDistance%20Between%20Meshes)) 10.684 0.0)) false))
                  (:==
                    (Components|InstancedStaticMesh|AddInstance (Variables|Default|GetEmptyTube) (Math|Transform|MakeTransform (Math|Vector|MakeVector (* (- (Variables|Default|GetTubesPlaced) 30) (Variables|Default|GetDistance%20Between%20Meshes)) 8.013 0.0)) false :!label _label_9))
                  (:<
                    (goto _label_9))))
              (:==
                (Components|InstancedStaticMesh|AddInstance (Variables|Default|GetEmptyTube) (Math|Transform|MakeTransform (Math|Vector|MakeVector (* (- (Variables|Default|GetTubesPlaced) 20) (Variables|Default|GetDistance%20Between%20Meshes)) 5.342 0.0)) false :!label _label_10))
              (:<
                (goto _label_10))))
          (:==
            (Components|InstancedStaticMesh|AddInstance (Variables|Default|GetEmptyTube) (Math|Transform|MakeTransform (Math|Vector|MakeVector (* (- (Variables|Default|GetTubesPlaced) 10) (Variables|Default|GetDistance%20Between%20Meshes)) 2.671 0.0)) false :!label _label_11))
          (:<
            (goto _label_11))))
      (:==
        (Components|InstancedStaticMesh|AddInstance (Variables|Default|GetEmptyTube) (Math|Transform|MakeTransform (Math|Vector|MakeVector (* (Variables|Default|GetTubesPlaced) (Variables|Default|GetDistance%20Between%20Meshes)) 0.0 0.0)) false :!label _label_12))
      (:<
        (goto _label_12)))))